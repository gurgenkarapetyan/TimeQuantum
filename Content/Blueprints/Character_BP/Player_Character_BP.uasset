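; Player character Blueprint handling axis movement and look, jumping, a dash and gun firing.
; BeginPlay spawns a knife and gun and attaches them to mesh sockets; only the gun is used here.
; Left Shift launches a moving, walking player along doubled velocity plus lift, with a Tick-timed cooldown.
; Firing plays a montage and sound, calls the gun's FireBullet, and blocks refiring for the montage's length before decrementing ammo.
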(event EventTick
  (params (DeltaSeconds :type Float%20%28single-precision%29))
  (Utilities|FlowControl|Sequence
    (:then_1
      ;[1 1 1] Dash Timer Interval.
      (if (not (Variables|Default|GetCanDash))
        (Variables|Default|SetDashTimer (+ (Variables|Default|GetDashTimer) DeltaSeconds))
        (if (>= (Variables|Default|GetDashTimer) (Variables|Default|GetDashInterval))
          (Variables|Default|SetDashTimer 0.0)
          (Variables|Default|SetCanDash true))))))

(event EventBeginPlay
  ;[1 1 1] Attach Weapons.
  (bind _returnvalue (Game|SpawnActorfromClass "/Game/Blueprints/Weapons_BP/Knife_BP.Knife_BP_C" (Transformation|GetSocketTransform (Variables|Character|GetMesh) "b_Knife" "RTS_World") "Undefined" 0 0))
  (bind _output_get (Variables|Default|SetKnife _returnvalue))
  (Transformation|AttachComponentToComponent _output_get (Variables|Character|GetMesh) "b_Knife" "KeepWorld" "KeepWorld" "KeepWorld" true)
  (bind _returnvalue_2 (Game|SpawnActorfromClass "/Game/Blueprints/Weapons_BP/Gun_BP.Gun_BP_C" (Transformation|GetSocketTransform (Variables|Character|GetMesh) "b_Gun" "RTS_World") "Undefined" 0 0))
  (bind _output_get_2 (Variables|Default|SetGun _returnvalue_2))
  (Transformation|AttachComponentToComponent _output_get_2 (Variables|Character|GetMesh) "b_Gun" "KeepWorld" "KeepWorld" "KeepWorld" true))

(event Input|ActionEvents|InputActionJump
  (params (Key :type Key%20Structure :default "None"))
  ;[1 1 1] Jump.
  (:Pressed
    (Character|Jump))
  (:Released
    (Character|StopJumping)))

(event Input|ActionEvents|InputActionFire
  (params (Key :type Key%20Structure :default "None"))
  ;[1 1 1] Shoot Gun
  (:Pressed
    (if (> (Variables|Default|GetCurrentAmmo) 0)
      (if (Variables|Default|GetCanPerformAction)
        (Variables|Default|SetCanPerformAction false)
        (bind _returnvalue (Animation|Montage|MontagePlay (Components|SkeletalMesh|GetAnimInstance (Variables|Character|GetMesh)) 0 1.0 "MontageLength" 0.0 true))
        (Audio|Components|Audio|Play (Variables|Default|GetGun%20Attack%20Sound) 0.0)
        (Default|FireBullet (Variables|Default|GetGun))
        (Utilities|FlowControl|Delay _returnvalue)
        (Math|Integer|DecrementInt (Variables|Default|GetCurrentAmmo)
          (:%20%20
            (Variables|Default|SetCanPerformAction true))))
      (else
        (Audio|Components|Audio|Play (Variables|Default|GetEmpty%20Gun%20Sound) 0.0)))))

(event Input|AxisEvents|InputAxisMoveForward
  (params (AxisValue :type Float%20%28single-precision%29))
  ;[1 1 1] Movement.
  (Pawn|Input|AddMovementInput (Transformation|GetActorForwardVector) AxisValue false))

(event Input|AxisEvents|InputAxisMoveRight
  (params (AxisValue :type Float%20%28single-precision%29))
  ;[1 1 1] Movement.
  (Pawn|Input|AddMovementInput (Transformation|GetActorRightVector) AxisValue false))

(event Input|AxisEvents|InputAxisTurn
  (params (AxisValue :type Float%20%28single-precision%29))
  ;[1 1 1] Rotation.
  (Pawn|Input|AddControllerYawInput AxisValue))

(event Input|AxisEvents|InputAxisLookUp
  (params (AxisValue :type Float%20%28single-precision%29))
  ;[1 1 1] Rotation.
  (Pawn|Input|AddControllerPitchInput AxisValue))

(event Input|KeyboardEvents|LeftShift
  (params (Key :type Key%20Structure :default "None"))
  (bind _returnvalue (Transformation|GetVelocity))
  (bind _returnvalue_2 (/ _returnvalue 0.5))
  (bind (_x _y _z) (Math|Vector|BreakVector _returnvalue_2))
  ;[1 1 1] Dash.
  (:Pressed
    (if (Math|Boolean|ANDBoolean (Class|KismetMathLibrary|NotEqualExactlyVectorVector (Transformation|GetVelocity) "0, 0, 0") (Variables|Default|GetCanDash) (Utilities|Enum|Equal(Enum) (Variables|/Script/Engine.CharacterMovementComponent|GetMovementMode (Variables|Character|GetCharacterMovement)) "MOVE_Walking"))
      (Character|LaunchCharacter (Math|Vector|MakeVector _x _y (+ _z 2e+02)) false false)
      (Variables|Default|SetCanDash false))))

(fn ConstructionScript)